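; BP_Chest is an interactable chest that grants coins once to the player character.
; CanInteract allows use only while unopened, and Interact also checks Opened before casting the caller to BP_ThirdPersonCharacter_Duplicate and adding CoinsToGive to its Coin.
; It then marks itself opened, snaps the SMTapa lid to a fixed world rotation without animation, and prints a Spanish debug message with the character's new coin total.
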(event `/Game/BluePrints/BPI_Interactable.Interact`
  (params (Caller :type "Actor Object Reference"))
  (if (not (`self.bOpened`))
    (bind _asbp_third_person_character_duplicate (cast `/Game/ThirdPerson/Blueprints/BP_ThirdPersonCharacter_Duplicate` Caller))
    (bind _output_get (set `/Game/ThirdPerson/Blueprints/BP_ThirdPersonCharacter_Duplicate.Coin` (+ (`/Game/ThirdPerson/Blueprints/BP_ThirdPersonCharacter_Duplicate.Coin` _asbp_third_person_character_duplicate) (`self.CoinsToGive`)) _asbp_third_person_character_duplicate))
    (`|ExecutionSequence`
      (:`then_0`
        (set `self.bOpened` true)
        (`SceneComponent.K2_SetWorldRotation` (`self.SM_Tapa`) (struct :`Pitch` 90.0) false false))
      (:`then_1`
        (bind _output_get_2 (set `/Game/ThirdPerson/Blueprints/BP_ThirdPersonCharacter_Duplicate.Coin` _output_get _asbp_third_person_character_duplicate))
        (`KismetSystemLibrary.PrintString` "Monedas que le dio el cofre")
        (`KismetSystemLibrary.PrintString` (`KismetStringLibrary.Conv_IntToString` _output_get_2))))))

(fn `CanInteract`
  (params (Caller :type "Actor Object Reference"))
  (returns (isInteract :type Boolean))
  (return (not (`self.bOpened`))))

(fn `UserConstructionScript`)