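; Player damage component that deals area damage in front of its owning actor when DealDamage is called.
; It runs a sphere overlap offset along the owner's forward vector by a fraction of Range, filtered by configured object types and excluding the owner.
; Each hit actor implementing BPI_Damage receives the component's Damage value through an interface message; the event's DamageAmount input is unused.
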(event `DealDamage`
  (params (DamageAmount :type Integer))
  (bind _returnvalue (`self.GetOwner`))
  (bind _returnvalue_2 (`self.GetOwner`))
  (set `self.DamageToApply` (`self.Damage`))
  (bind _outactors (`KismetSystemLibrary.SphereOverlapActors` (+ (`Actor.K2_GetActorLocation` _returnvalue) (* (* (`self.Range`) 0.7) (`Actor.GetActorForwardVector` _returnvalue))) (`self.Radius`) (`self.ObjectTypesToHit`) null (`|MakeArray` _returnvalue_2)))
  (for _array_element _outactors
    (if (!= _array_element _returnvalue_2)
      (if (`KismetSystemLibrary.DoesImplementInterface` _array_element "/Game/BluePrints/BPI_Damage.BPI_Damage_C")
        (message `/Game/BluePrints/BPI_Damage.RecieveDamage` _array_element (`self.DamageToApply`))))))