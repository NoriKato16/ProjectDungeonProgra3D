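; BP_SpikeTrap is a spike trap actor that hurts the player character on overlap while armed.
; Spikes start lowered by a Z offset at BeginPlay, and ArmTrap and DisarmTrap toggle Active and ease them between raised and hidden positions.
; Overlapping Collision while Active calls ReceiveDamage on the character's health component.
; CanInteract always returns true; the delay after arming leads to an empty branch, so nothing auto-retracts.
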(event `self.ReceiveBeginPlay`
  (bind _output_get (set `self.RaisedLocation` (`SceneComponent.RelativeLocation` (`self.Spikes`))))
  (bind _output_get_2 (set `self.HiddenLocation` (+ _output_get (`KismetMathLibrary.MakeVector` 0.0 0.0 (`self.HiddenOffsetZ`)))))
  (`SceneComponent.K2_SetRelativeLocation` (`self.Spikes`) _output_get_2 false false))

(event `self.Collision.OnComponentBeginOverlap`
  (params (OverlappedComponent :type "PrimitiveComponent Object Reference") (OtherActor :type "Actor Object Reference") (OtherComp :type "PrimitiveComponent Object Reference") (OtherBodyIndex :type Integer) (bFromSweep :type Boolean) (SweepResult :type "HitResult Structure (by ref)"))
  (if (`self.bActive`)
    (bind _asbp_third_person_character_duplicate (cast `/Game/ThirdPerson/Blueprints/BP_ThirdPersonCharacter_Duplicate` OtherActor))
    (`HealthSystemComponent.ReceiveDamage` (`/Game/ThirdPerson/Blueprints/BP_ThirdPersonCharacter_Duplicate.BPC_HealthSystemComponent` _asbp_third_person_character_duplicate))
    (`KismetSystemLibrary.PrintString` "recieved damage")))

(event `ArmTrap`
  (set `self.bActive` true)
  (`KismetSystemLibrary.MoveComponentTo` (`self.Spikes`) (`self.RaisedLocation`) (struct) true true (`self.MoveTime`))
  (`KismetSystemLibrary.Delay` (`self.RetractDelay`))
  (if (`self.bActive`)
    _))

(event `DisarmTrap`
  (bind _movetime (`self.MoveTime`))
  (set `self.bActive` false)
  (`KismetSystemLibrary.MoveComponentTo` (`self.Spikes`) (`self.HiddenLocation`) (struct) true true _movetime)
  (`KismetSystemLibrary.Delay` _movetime))

(fn `CanInteract`
  (params (Caller :type "Actor Object Reference"))
  (returns (isInteract :type Boolean))
  (return true))

(fn `UserConstructionScript`)