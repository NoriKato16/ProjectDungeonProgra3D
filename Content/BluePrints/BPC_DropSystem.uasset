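; Drop component that awards coins to the dungeon game's running total, with no pickup actor spawned.
; Its DropCoin event uses the IsDropped flag to pay out only once, adding its Coins value to CoinsCollected on BP_DungeonGameMode.
; The new total is printed to screen, and BeginPlay and Tick are unused.
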(event `DropCoin`
  (if (not (`self.IsDropped`))
    (set `self.IsDropped` true)
    (bind _asbp_dungeon_game_mode (cast `/Game/BluePrints/BP_DungeonGameMode` (`GameplayStatics.GetGameMode`)))
    (bind _output_get (set `/Game/BluePrints/BP_DungeonGameMode.CoinsCollected` (+ (`/Game/BluePrints/BP_DungeonGameMode.CoinsCollected` _asbp_dungeon_game_mode) (`self.Coins`)) _asbp_dungeon_game_mode))
    (`KismetSystemLibrary.PrintString` (`KismetStringLibrary.Conv_IntToString` _output_get))))