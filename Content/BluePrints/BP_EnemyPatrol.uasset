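; BP_EnemyPatrol is an enemy character that deals contact damage to the player and can be killed; this graph holds no patrol movement.
; On Hit, it calls ReceiveDamage on the player character's health component, then blocks further damage until a cooldown timer resets CanDamage.
; Its RecieveDamage event decrements its own Health; at zero, Die unpossesses it, ragdolls the mesh and sets a short lifespan.
; CanInteract always returns true.
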(event `self.ReceiveActorBeginOverlap`
  (params (OtherActor :type "Actor Object Reference")))

(event `self.ReceiveHit`
  (params (MyComp :type "PrimitiveComponent Object Reference") (Other :type "Actor Object Reference") (OtherComp :type "PrimitiveComponent Object Reference") (bSelfMoved :type Boolean) (HitLocation :type "Vector Structure") (HitNormal :type "Vector Structure") (NormalImpulse :type "Vector Structure") (Hit :type "HitResult Structure (by ref)"))
  (if true
    (if (`self.CanDamage`)
      (bind _asbp_third_person_character_duplicate (cast `/Game/ThirdPerson/Blueprints/BP_ThirdPersonCharacter_Duplicate` Other))
      (`HealthSystemComponent.ReceiveDamage` (`/Game/ThirdPerson/Blueprints/BP_ThirdPersonCharacter_Duplicate.BPC_HealthSystemComponent` _asbp_third_person_character_duplicate))
      (set `self.CanDamage` false)
      (`KismetSystemLibrary.K2_SetTimer` null "ResetCanDamage" (`self.DamageCooldown`)))))

(event `/Game/BluePrints/BPI_Damage.RecieveDamage`
  (params (Damage :type Integer))
  (bind _output_get (set `self.Health` (+ (`self.Health`) -1)))
  (if (<= _output_get 0)
    (`self.Die`)))

(fn `CanInteract`
  (returns (isInteract :type Boolean))
  (return true))

(fn `Die`
  (`MovementComponent.StopMovementImmediately` (`self.CharacterMovement`))
  (`Controller.UnPossess` (`self.GetController`))
  (`PrimitiveComponent.SetCollisionEnabled` (`self.CapsuleComponent`) "NoCollision")
  (`PrimitiveComponent.SetCollisionProfileName` (`self.Mesh`) "Ragdoll" true)
  (`SkeletalMeshComponent.SetAllBodiesSimulatePhysics` (`self.Mesh`) true)
  (`PrimitiveComponent.SetSimulatePhysics` (`self.Mesh`) true)
  (`SkeletalMeshComponent.SetAllBodiesBelowPhysicsBlendWeight` (`self.Mesh`) (`self.In Bone Name`) 1.0 false true)
  (`PrimitiveComponent.WakeAllRigidBodies` (`self.Mesh`))
  (`self.SetLifeSpan` 2.0))

(fn `ResetCanDamage`
  (set `self.CanDamage` true))

(fn `UserConstructionScript`)