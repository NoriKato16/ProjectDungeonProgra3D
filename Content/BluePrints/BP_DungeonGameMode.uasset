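; Dungeon game mode Blueprint that tracks collected coins and handles win and lose outcomes.
; AddCoin increments the count and calls WinGame at exactly VictoryCoins, which flags game over and calls OpenLevelByName with an unset "None" level.
; AddScore separately adds a given amount and only prints the total or a win message.
; PlayerDied calls LoseGame, which only prints text without setting the game-over flag.
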(event `AddScore`
  (params (CoinToAdd :type Integer))
  (bind _output_get (set `self.CoinsCollected` (+ CoinToAdd (`self.CoinsCollected`))))
  (bind _returnvalue (`KismetStringLibrary.Conv_IntToString` _output_get))
  (`KismetSystemLibrary.PrintString` (select `bool` (>= _output_get (`self.VictoryCoins`)) :`false` _returnvalue :`true` (`KismetStringLibrary.Concat_StrStr` "Ganaste" _returnvalue))))

(fn `AddCoin`
  (bind _output_get (set `self.CoinsCollected` (+ (`self.CoinsCollected`) 1)))
  (if (== _output_get (`self.VictoryCoins`))
    (`self.WinGame`)))

(fn `LoseGame`
  (`KismetSystemLibrary.PrintText` "You Lose"))

(fn `PlayerDied`
  (`KismetSystemLibrary.PrintString` "in playerdied")
  (`self.LoseGame`)
  (`KismetSystemLibrary.PrintString` "Lose game"))

(fn `UserConstructionScript`)

(fn `WinGame`
  (set `self.IsGameOver` true)
  (`KismetSystemLibrary.PrintText` "You Win, opening next level")
  (`GameplayStatics.OpenLevel` "None"))