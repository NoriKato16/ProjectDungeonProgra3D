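; Behavior tree task that makes an AI attack the player character stored in the blackboard's target key.
; On execute it casts the target to the third-person character and calls ReceiveDamage on its health component.
; A timer-reset flag enforces a cooldown between hits, and the task fails while on cooldown.
; A failed cast leaves the task without finishing.
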(event `self.ReceiveExecuteAI`
  (params (OwnerController :type "AIController Object Reference") (ControlledPawn :type "Pawn Object Reference"))
  (bind _asbp_third_person_character_duplicate (cast `/Game/ThirdPerson/Blueprints/BP_ThirdPersonCharacter_Duplicate` (`BlackboardComponent.GetValueAsObject` (`AIController.Blackboard` OwnerController) (`self.TargetActor`))))
  (if (`self.CanDamage`)
    (`HealthSystemComponent.ReceiveDamage` (`Actor.GetComponentByClass` _asbp_third_person_character_duplicate "/Game/BluePrints/BPC_HealthSystemComponent.BPC_HealthSystemComponent_C"))
    (set `self.CanDamage` false)
    (`KismetSystemLibrary.K2_SetTimer` null "ResetCanDamage" (`self.CoolDown`))
    (`self.FinishExecute` true)
    (else
      (`self.FinishExecute` false))))

(event `ResetCanDamage`
  (set `self.CanDamage` true))