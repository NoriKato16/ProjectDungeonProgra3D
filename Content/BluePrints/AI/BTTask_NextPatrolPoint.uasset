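; Behavior tree task that advances an enemy to the next patrol point in its route.
; It increments its own CurrentPatrolIndex, wrapping around the controlled enemy's PatrolPoints array, and writes that actor's location to the PatrolLocationKey blackboard entry.
; It relies on BP_EnemyPatrolController for the enemy and blackboard, finishing successfully after the write but never finishing if that cast fails.
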(event `self.ReceiveExecuteAI`
  (params (OwnerController :type "AIController Object Reference") (ControlledPawn :type "Pawn Object Reference"))
  (bind _asbp_enemy_patrol_controller (cast `/Game/BluePrints/BP_EnemyPatrolController` OwnerController))
  (bind _patrolpoints (`/Game/BluePrints/BP_EnemyPatrol.PatrolPoints` (`/Game/BluePrints/BP_EnemyPatrolController.ControlledEnemy` _asbp_enemy_patrol_controller)))
  (bind _output_get (set `self.CurrentPatrolIndex` (mod (+ (`self.CurrentPatrolIndex`) 1) (`KismetArrayLibrary.Array_Length` _patrolpoints))))
  (`BlackboardComponent.SetValueAsVector` (`/Game/BluePrints/BP_EnemyPatrolController.BlackBoardComp` _asbp_enemy_patrol_controller) (`self.PatrolLocationKey`) (`Actor.K2_GetActorLocation` (`|GetArrayItem` _patrolpoints _output_get)))
  (`self.FinishExecute` true))