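; BP_RangedEnemy is an AI-controlled ranged enemy that fires projectiles at the player character and reports its team through GetTeam.
; ShootAtLastLocation reads TargetActor from its controller's blackboard, then spawns a BP_Projectile at the spawn point, aimed at that actor's current location despite the function's name.
; It sets the projectile velocity along that direction using ProjectileSpeed and plays a shot sound.
; The event graph has no active logic.
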(fn `GetTeam`
  (returns (Team :type "/BPP_SimpleTeamPlugin/Teams/E_Team Enum"))
  (return "NewEnumerator2"))

(fn `ShootAtLastLocation`
  (bind _returnvalue (`SceneComponent.K2_GetComponentLocation` (`self.ProjectileSpawnPoint`)))
  (bind _asbp_ranged_enemy_controller (cast `/Game/BluePrints/AI/RangedEnemy/BP_RangedEnemyController` (`self.GetController`)))
  (bind _asbp_third_person_character_duplicate (cast `/Game/ThirdPerson/Blueprints/BP_ThirdPersonCharacter_Duplicate` (`BlackboardComponent.GetValueAsObject` (`/Game/BluePrints/AI/RangedEnemy/BP_RangedEnemyController.BlackBoardComp` _asbp_ranged_enemy_controller) (`self.TargetActor`))))
  (bind _returnvalue_2 (`KismetMathLibrary.Normal` (`KismetMathLibrary.GetDirectionUnitVector` _returnvalue (`self.K2_GetActorLocation` _asbp_third_person_character_duplicate))))
  (bind _returnvalue_3 (`|SpawnActorFromClass` "/Game/BluePrints/AI/RangedEnemy/BP_Projectile.BP_Projectile_C" (`KismetMathLibrary.MakeTransform` _returnvalue (`KismetMathLibrary.MakeRotFromX` _returnvalue_2)) "AlwaysSpawn" "MultiplyWithRoot" null null))
  (set `MovementComponent.Velocity` (* _returnvalue_2 (`self.ProjectileSpeed`)) (`/Game/BluePrints/AI/RangedEnemy/BP_Projectile.ProjectileMovement` _returnvalue_3))
  (`GameplayStatics.PlaySoundAtLocation` "/Game/Audio/Cues/SC_Shoot.SC_Shoot" (`self.K2_GetActorLocation`) (struct) 1.0 1.0 0.0 null null null null))

(fn `UserConstructionScript`
  (`parent.UserConstructionScript`))