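; BP_PushableObject is a stone coffin mesh the player character can move in four directions.
; The Fwd component's overlap events toggle the character's CanInteractBox flag, without checking which actor overlaps.
; While that flag and IsInteractingBox are true, Tick reads the character's input axes and calls Speed/Direction.
; That function nudges the mesh along its forward or right vector using VInterpTo, without sweep, and debug prints trace each state.
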(event `self.ReceiveBeginPlay`
  (bind _returnvalue (`GameplayStatics.GetActorOfClass` "/Game/ThirdPerson/Blueprints/BP_ThirdPersonCharacter_Duplicate.BP_ThirdPersonCharacter_Duplicate_C"))
  (set `self.CharRef` _returnvalue))

(event `self.ReceiveTick`
  (params (DeltaSeconds :type "Float (single-precision)"))
  (bind _charref (`self.CharRef`))
  (bind _charref_2 (`self.CharRef`))
  (bind _forward_back_axis (`/Game/ThirdPerson/Blueprints/BP_ThirdPersonCharacter_Duplicate.Forward Back Axis` _charref_2))
  (bind _left_right_axis (`/Game/ThirdPerson/Blueprints/BP_ThirdPersonCharacter_Duplicate.Left Right Axis` _charref_2))
  (if (`/Game/ThirdPerson/Blueprints/BP_ThirdPersonCharacter_Duplicate.IsInteractingBox` _charref)
    (if (`/Game/ThirdPerson/Blueprints/BP_ThirdPersonCharacter_Duplicate.CanInteractBox` _charref)
      (`|ExecutionSequence`
        (:`then_0`
          (if (== _forward_back_axis 0.0)
            (`KismetSystemLibrary.PrintString` "Player not moving fwd/bck" true true (struct :`R` 1.0 :`B` 0.861054 :`A` 1.0) 2.0 "1111")
            (elif (> _forward_back_axis 0.0)
              (`KismetSystemLibrary.PrintString` "Moving forward" true true (struct :`R` 1.0 :`G` 0.933289 :`A` 1.0) 2.0 "4444")
              (`self.Speed/Direction` true -34.0)
              (else
                (`KismetSystemLibrary.PrintString` "Moving backwards" true true (struct :`R` 1.0 :`G` 0.933289 :`A` 1.0) 2.0 "3333")
                (`self.Speed/Direction` true 34.0)))))
        (:`then_1`
          (if (== _left_right_axis 0.0)
            (`KismetSystemLibrary.PrintString` "Player not moving sides" true true (struct :`R` 1.0 :`B` 0.861054 :`A` 1.0) 2.0 "23545")
            (elif (> _left_right_axis 0.0)
              (`KismetSystemLibrary.PrintString` "Moving right" true true (struct :`R` 1.0 :`G` 0.933289 :`A` 1.0) 2.0 "457567")
              (`self.Speed/Direction` false -34.0)
              (else
                (`KismetSystemLibrary.PrintString` "Moving left" true true (struct :`R` 1.0 :`G` 0.933289 :`A` 1.0) 2.0 "76678")
                (`self.Speed/Direction` false 34.0)))))))))

(event `self.Fwd.OnComponentBeginOverlap`
  (params (OverlappedComponent :type "PrimitiveComponent Object Reference") (OtherActor :type "Actor Object Reference") (OtherComp :type "PrimitiveComponent Object Reference") (OtherBodyIndex :type Integer) (bFromSweep :type Boolean) (SweepResult :type "HitResult Structure (by ref)"))
  (`KismetSystemLibrary.PrintString` "CanPush")
  (set `/Game/ThirdPerson/Blueprints/BP_ThirdPersonCharacter_Duplicate.CanInteractBox` true (`self.CharRef`)))

(event `self.Fwd.OnComponentEndOverlap`
  (params (OverlappedComponent :type "PrimitiveComponent Object Reference") (OtherActor :type "Actor Object Reference") (OtherComp :type "PrimitiveComponent Object Reference") (OtherBodyIndex :type Integer))
  (`KismetSystemLibrary.PrintString` "CantPush")
  (set `/Game/ThirdPerson/Blueprints/BP_ThirdPersonCharacter_Duplicate.CanInteractBox` false (`self.CharRef`)))

(fn `UserConstructionScript`)